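; BP_Brush is a snow brush that reports where its owner presses into the snow to the level's BP_PaintBoard.
; It finds and caches the paint board on BeginPlay.
; Each tick it traces down on the Visibility channel from its Z-offset world location over the snow height.
; On a hit, it sends that start position, the brush size and the hit distance as height via AddBrushInfo.
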(event `self.ReceiveBeginPlay`
  (bind _returnvalue (`GameplayStatics.GetActorOfClass` "/Game/Snow/BP_PaintBoard.BP_PaintBoard_C"))
  ;[1 1 1] 提升变量，避免重复获取
  (set `self.PaintBoard` _returnvalue))

(event `self.ReceiveTick`
  (params (DeltaSeconds :type "Float (single-precision)"))
  (bind _returnvalue (- (`self.K2_GetComponentLocation`) (`KismetMathLibrary.MakeVector` 0.0 0.0 (`self.Zoffset`))))
  (bind (_outhit _returnvalue_2) (`KismetSystemLibrary.LineTraceSingle` _returnvalue (- _returnvalue (`KismetMathLibrary.MakeVector` 0.0 0.0 (`self.SnowHeight`))) "TraceTypeQuery1"))
  (if _returnvalue_2
    (`/Game/Snow/BP_PaintBoard.AddBrushInfo` (`self.PaintBoard`) (make `/Game/Snow/S_BrushInfo` _returnvalue (`self.Size`) (`.Distance` (`GameplayStatics.BreakHitResult` _outhit))))))