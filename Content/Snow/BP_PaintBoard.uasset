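; Snow deformation paint board that keeps a render-target height map centered on the player.
; Each tick it snaps to the texel grid, publishes position and size to MPC_Snow, then copies RT_Snow and redraws it shifted by the movement via a translation material.
; Queued brush infos are stamped with M_Draw by position, size and height, then cleared, and M_Pile is drawn into RT_SnowSave.
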(event `self.ReceiveBeginPlay`
  (bind (_size_x _size_y) (`KismetMathLibrary.BreakVector2D` (`self.Size`)))
  (bind (_position_x _position_y) (`KismetMathLibrary.BreakVector2D` (`self.Position`)))
  (`KismetRenderingLibrary.ClearRenderTarget2D` "/Game/Snow/RT_Snow.RT_Snow")
  (set `self.PixelSize` (/ (`self.Size`) (`self.分辨率`)))
  (`KismetMaterialLibrary.SetVectorParameterValue` "/Game/Snow/MPC_Snow.MPC_Snow" "PositionSize" (make `LinearColor` _position_x _position_y _size_x _size_y)))

(event `self.ReceiveTick`
  (params (DeltaSeconds :type "Float (single-precision)"))
  (`self.UpdatePos` (`KismetMathLibrary.Conv_VectorToVector2D` (`self.K2_GetActorLocation` (`GameplayStatics.GetPlayerPawn` 0))))
  ;[1 1 1] 将RT拷贝为RTsave
  (`self.CopyRT`)
  (`KismetRenderingLibrary.ClearRenderTarget2D` "/Game/Snow/RT_Snow.RT_Snow")
  ;[1 1 1] 将RTsave以M_Translation平移，将动态材质实例写入到RT中
  (bind _returnvalue (`KismetMaterialLibrary.CreateDynamicMaterialInstance` "/Game/Snow/M_Traslation.M_Traslation"))
  (`self.设置平移参数` _returnvalue)
  (`KismetRenderingLibrary.DrawMaterialToRenderTarget` "/Game/Snow/RT_Snow.RT_Snow" _returnvalue)
  (`self.Draw`)
  (`KismetRenderingLibrary.DrawMaterialToRenderTarget` "/Game/Snow/RT_SnowSave.RT_SnowSave" "/Game/Snow/M_Pile.M_Pile"))

(event `AddBrushInfo`
  (params (Info :type "/Game/Snow/S_BrushInfo Structure"))
  (`KismetArrayLibrary.Array_Add` (`self.Infos`) Info))

(fn `CopyRT`
  (bind (_canvas _size _context) (`KismetRenderingLibrary.BeginDrawCanvasToRenderTarget` "/Game/Snow/RT_SnowSave.RT_SnowSave"))
  (`Canvas.K2_DrawTexture` _canvas "/Game/Snow/RT_Snow.RT_Snow" (0.0 0.0) _size (0.0 0.0) (1.0 1.0) (struct :`R` 1.0 :`G` 1.0 :`B` 1.0 :`A` 1.0) "BLEND_Opaque" 0.0 (0.5 0.5))
  (`KismetRenderingLibrary.EndDrawCanvasToRenderTarget` _context))

(fn `Draw`
  (bind _snowheight (`self.SnowHeight`))
  (bind _returnvalue (`KismetMaterialLibrary.CreateDynamicMaterialInstance` "/Game/Snow/M_Draw.M_Draw"))
  (`self.设置平移参数` _returnvalue)
  (bind (_canvas _size _context) (`KismetRenderingLibrary.BeginDrawCanvasToRenderTarget` "/Game/Snow/RT_Snow.RT_Snow"))
  (for _array_element (`self.Infos`)
    (bind (_position _size_2 _height) (break `/Game/Snow/S_BrushInfo` _array_element))
    (`MaterialInstanceDynamic.SetScalarParameterValue` _returnvalue "Height" (- 1.0 (/ (- _snowheight _height) _snowheight)))
    (bind _returnvalue_2 (/ _size_2 (`self.PixelSize`)))
    (`Canvas.K2_DrawMaterial` _canvas _returnvalue (- (* _size (`self.WorldToUV` _position)) (/ _returnvalue_2 (2.0 2.0))) _returnvalue_2 (0.0 0.0) (1.0 1.0) 0.0 (0.5 0.5)))
  (`KismetRenderingLibrary.EndDrawCanvasToRenderTarget` _context)
  (`KismetArrayLibrary.Array_Clear` (`self.Infos`)))

(fn `UpdatePos`
  (params (Position :type "Vector2D Structure"))
  (bind (_position_x _position_y) (`KismetMathLibrary.BreakVector2D` (`self.Position`)))
  (bind (_size_x _size_y) (`KismetMathLibrary.BreakVector2D` (`self.Size`)))
  (bind _returnvalue (/ (`self.Size`) (`self.分辨率`)))
  (bind (_returnvalue_x _returnvalue_y) (`KismetMathLibrary.BreakVector2D` (/ Position _returnvalue)))
  ;[1 1 1] Update Position & Set LastLoc& Pixels
  (set `self.LastLocation` (`self.Position`))
  (set `self.Position` (* _returnvalue (`KismetMathLibrary.MakeVector2D` (`KismetMathLibrary.Conv_IntToDouble` (`KismetMathLibrary.FFloor` _returnvalue_x)) (`KismetMathLibrary.Conv_IntToDouble` (`KismetMathLibrary.FFloor` _returnvalue_y)))))
  ;[1 1 1] DEBUG
  (`SceneComponent.K2_SetWorldTransform` (`self.Plane`) (`KismetMathLibrary.MakeTransform` (`KismetMathLibrary.Conv_Vector2DToVector` (`self.Position`)) (struct) (`KismetMathLibrary.Conv_Vector2DToVector` (/ (`self.Size`) (100.0 100.0)))) false false)
  ;[1 1 1] MPC
  (`KismetMaterialLibrary.SetVectorParameterValue` "/Game/Snow/MPC_Snow.MPC_Snow" "PositionSize" (make `LinearColor` _position_x _position_y _size_x _size_y)))

(fn `UserConstructionScript`
  (`SceneComponent.K2_SetWorldTransform` (`self.Plane`) (`KismetMathLibrary.MakeTransform` (`KismetMathLibrary.Conv_Vector2DToVector` (`self.Position`)) (struct) (`KismetMathLibrary.Conv_Vector2DToVector` (/ (`self.Size`) (100.0 100.0)))) false false))

(fn `WorldToUV`
  (params (Position :type "Vector Structure"))
  (returns (ReturnValue :type "Vector2D Structure"))
  (return (+ (/ (- (`KismetMathLibrary.MakeVector2D` (.x Position) (.y Position)) (`self.Position`)) (`self.Size`)) (0.5 0.5))))

(fn `设置平移参数`
  (params (self2 :type "MaterialInstanceDynamic Object Reference"))
  (bind (_x _y) (`KismetMathLibrary.BreakVector2D` (/ (- (`self.Position`) (`self.LastLocation`)) (`self.Size`))))
  (`MaterialInstanceDynamic.SetVectorParameterValue` self2 "Offset" (make `LinearColor` _x _y)))